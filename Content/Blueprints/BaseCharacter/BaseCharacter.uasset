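; Base first-person character that moves, looks, jumps, interacts with objects and carries one item at a time.
; BeginPlay creates the HUD widget and sets the character as its owner.
; Use line-traces from the camera and calls Interact on every Interactable component of the hit actor.
; PickUp attaches an actor to the Hand socket with collision, physics and gravity off; Drop detaches it and restores them.
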(event `InputAxis|Forward`
  (params (AxisValue :type "Float (single-precision)"))
  ;[1 1 1] Movement
  (`self.AddMovementInput` (`self.GetActorForwardVector`) AxisValue))

(event `InputAxis|Look Down`
  (params (AxisValue :type "Float (single-precision)"))
  ;[1 1 1] Looking around
  (`self.AddControllerPitchInput` AxisValue))

(event `self.ReceiveBeginPlay`
  ;[1 1 1] HUD setup
  (bind _returnvalue (`|CreateWidget` "/Game/Blueprints/BaseCharacter/HUD.HUD_C" (`GameplayStatics.GetPlayerController` 0)))
  (bind _output_get (set `self.HUD` _returnvalue))
  (`UserWidget.AddToViewport` _output_get 0)
  (set `/Game/Blueprints/BaseCharacter/HUD.Owner` self _output_get))

(event `InputAxis|Look Right`
  (params (AxisValue :type "Float (single-precision)"))
  ;[1 1 1] Looking around
  (`self.AddControllerYawInput` AxisValue))

(event `InputAxis|Right`
  (params (AxisValue :type "Float (single-precision)"))
  ;[1 1 1] Movement
  (`self.AddMovementInput` (`self.GetActorRightVector`) AxisValue))

(event `InputAction|Jump`
  (params (Key :type "Key Structure" :default "AnyKey"))
  ;[1 1 1] Movement
  (:`Pressed`
    (`self.Jump`)))

(event `InputAction|Use`
  (params (Key :type "Key Structure" :default "AnyKey"))
  (bind (_found _success) (`self.Get Facing Actor` 2000))
  ;[1 1 1] Interaction
  (:`Pressed`
    (if _success
      (for _array_element (`self.K2_GetComponentsByClass` _found "/Game/Blueprints/Components/Interactable.Interactable_C")
        (`/Game/Blueprints/Components/Interactable.Interact` _array_element self)))))

(event `InputAction|Drop`
  (params (Key :type "Key Structure" :default "AnyKey"))
  ;[1 1 1] Drop stuff
  (:`Pressed`
    (`self.Drop Item`)))

(fn `Drop Item`
  (bind _held_item (`self.Held Item`))
  (if (`self.Is Holding Item`)
    (`|ExecutionSequence`
      (:`then_0`
        (`self.DetachRootComponentFromParent` _held_item true))
      (:`then_1`
        (`self.SetActorEnableCollision` _held_item true))
      (:`then_2`
        (bind _asprimitive_component (cast `PrimitiveComponent` (`self.K2_GetRootComponent` _held_item)))
        (`|ExecutionSequence`
          (:`then_0`
            (`PrimitiveComponent.SetEnableGravity` _asprimitive_component true))
          (:`then_1`
            (`PrimitiveComponent.SetSimulatePhysics` _asprimitive_component true))))
      (:`then_3`
        (set `self.Is Holding Item` false)
        (set `self.Held Item` null)))))

(fn `Get Facing`
  (params (Distance :type Integer))
  (returns (Hit :type "HitResult Structure") (Sucess :type Boolean))
  (bind _firstpersoncamera (`self.FirstPersonCamera`))
  (bind _returnvalue (`SceneComponent.K2_GetComponentLocation` _firstpersoncamera))
  (bind (_outhit _returnvalue_2) (`KismetSystemLibrary.LineTraceSingle` _returnvalue (+ _returnvalue (* (`SceneComponent.GetForwardVector` _firstpersoncamera) Distance)) "TraceTypeQuery1"))
  (return _outhit _returnvalue_2))

(fn `Get Facing Actor`
  (params (Distance :type Integer))
  (returns (Found :type "Actor Object Reference") (Success :type Boolean))
  (bind (_hit _sucess) (`self.Get Facing` Distance))
  (if _sucess
    (return (`.HitActor` (`GameplayStatics.BreakHitResult` _hit)) true)
    (else
      (return null false))))

(fn `Get Facing Component`
  (params (Distance :type Integer))
  (returns (Component :type "PrimitiveComponent Object Reference") (Success :type Boolean))
  (return null (`.Sucess` (`self.Get Facing` Distance))))

(fn `Pick Up`
  (params (Actor :type "Actor Object Reference"))
  (bind _hand (`self.Hand`))
  (if (not (`self.Is Holding Item`))
    (`|ExecutionSequence`
      (:`then_0`
        (`self.K2_AttachRootComponentTo` Actor _hand "Hand" "KeepWorldPosition" true)
        (`KismetSystemLibrary.PrintString` "hi"))
      (:`then_1`
        (`self.K2_SetActorLocation` Actor (`SceneComponent.GetSocketLocation` _hand "Hand") false false)
        (`self.SetActorEnableCollision` Actor false)
        (bind _asprimitive_component (cast `PrimitiveComponent` (`self.K2_GetRootComponent` Actor)))
        (`PrimitiveComponent.SetSimulatePhysics` _asprimitive_component false)
        (`PrimitiveComponent.SetEnableGravity` _asprimitive_component false))
      (:`then_2`
        (set `self.Is Holding Item` true)
        (set `self.Held Item` Actor)))))

(fn `UserConstructionScript`)