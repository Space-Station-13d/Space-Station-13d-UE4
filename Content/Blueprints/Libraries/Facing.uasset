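; Function library that finds what lies straight ahead of a given transform within a given distance.
; Get Facing runs a Visibility line trace from the transform's location along its forward vector and returns the hit with a success flag.
; Get Facing Actor and Get Facing Component build on that trace to return the hit actor or component with success, the actor version branching on whether the trace hit.
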(fn `Get Facing`
  (params (Distance :type "Float (double-precision)") (Transform :type "Transform Structure (by ref)"))
  (returns (Hit :type "HitResult Structure") (Sucess :type Boolean))
  (bind _location (.location Transform))
  (bind (_outhit _returnvalue) (`KismetSystemLibrary.LineTraceSingle` null _location (+ _location (* (`KismetMathLibrary.GetForwardVector` (.rotation Transform)) Distance)) "TraceTypeQuery1"))
  (return _outhit _returnvalue))

(fn `Get Facing Actor`
  (params (Distance :type "Float (double-precision)") (Transform :type "Transform Structure (by ref)"))
  (returns (Found :type "Actor Object Reference") (Success :type Boolean))
  (bind (_hit _sucess) (`self.Get Facing` Distance Transform))
  (if _sucess
    (return (`.HitActor` (`GameplayStatics.BreakHitResult` _hit)) true)
    (else
      (return null false))))

(fn `Get Facing Component`
  (params (Distance :type "Float (double-precision)") (Transform :type "Transform Structure (by ref)"))
  (returns (Component :type "PrimitiveComponent Object Reference") (Success :type Boolean))
  (bind (_hit _sucess) (`self.Get Facing` Distance Transform))
  (return (`.HitComponent` (`GameplayStatics.BreakHitResult` _hit)) _sucess))