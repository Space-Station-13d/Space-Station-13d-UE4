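; A button actor that toggles nearby light fixtures when a player interacts with it.
; On BeginPlay, only on the authority, it collects every LightFixture within a fixed radius into its Lamp array and binds Toggle to its Interactable's OnInteracted event.
; Each interaction calls Toggle on every cached fixture, so the linked lights are found by proximity once at startup.
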(event `self.ReceiveBeginPlay`
  (`/Engine/EditorBlueprintResources/ActorMacros.Switch Has Authority`
    (:`Authority`
      (`|ExecutionSequence`
        (:`then_0`
          (bind _outactors (`GameplayStatics.GetAllActorsOfClass` "/Game/Blueprints/Game/LightFixture.LightFixture_C"))
          (for _array_element _outactors
            (if (<= (`KismetMathLibrary.VSize` (- (`self.K2_GetActorLocation` _array_element) (`self.K2_GetActorLocation`))) 10000.0)
              (`KismetArrayLibrary.Array_Add` (`self.Lamp`) _array_element))))
        (:`then_1`
          (add `/Game/Blueprints/Components/Interactable.OnInteracted` (`self.Interactable`) (delegate `Toggle`)))))))

(event `Toggle`
  (params (User :type "/Game/Blueprints/Mob/BaseCharacter Object Reference"))
  (for _array_element (`self.Lamp`)
    (`/Game/Blueprints/Game/LightFixture.Toggle` _array_element)))

(fn `UserConstructionScript`)