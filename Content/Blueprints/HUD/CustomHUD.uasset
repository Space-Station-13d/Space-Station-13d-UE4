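; CustomHUD is a HUD Blueprint that spawns and tracks the player's on-screen widgets.
; On BeginPlay it reads the widget class list from the first player's BasePlayerController, creates each widget, adds it to the viewport and stores it in the Widgets array.
; GetWidgetByClass searches that array and returns the first widget whose class exactly matches the requested one.
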(event `self.ReceiveBeginPlay`
  (bind _returnvalue (`GameplayStatics.GetPlayerController` 0))
  (bind _asbase_player_controller (cast `/Game/Blueprints/PlayerController/BasePlayerController` _returnvalue))
  (for _array_element (`/Game/Blueprints/PlayerController/BasePlayerController.GetHudClasses` _asbase_player_controller)
    (bind _returnvalue_2 (`|CreateWidget` _array_element _returnvalue))
    (`/Engine/EditorBlueprintResources/StandardMacros.IsValid` _returnvalue_2
      (:`Is Valid`
        (`KismetArrayLibrary.Array_Add` (`self.Widgets`) _returnvalue_2)
        (`UserWidget.AddToViewport` _returnvalue_2 0)))))

(fn `Get Widget By Class`
  (params (Class :type "UserWidget Class Reference"))
  (returns (Found :type "UserWidget Object Reference"))
  (for _array_element (`self.Widgets`)
    (if (== (`GameplayStatics.GetObjectClass` _array_element) Class)
      (return _array_element)))
  (return null))

(fn `UserConstructionScript`)