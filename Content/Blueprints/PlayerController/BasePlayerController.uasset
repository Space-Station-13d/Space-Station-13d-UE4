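; Base player controller that handles text chat and supplies the widget classes for the HUD.
; The Chat input focuses the CustomHUD's Chat widget in UI-only mode, and entered messages go to every BasePlayerController, which passes them to its own Chat widget.
; Messages are prefixed with a random "Player-" name assigned in the construction script.
; GetHudClasses combines the controlled BaseCharacter's widget classes with the controller's own HUDClasses.
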(event Custom|Chat%20Entered
  (params (Message :type Text))
  (bind _outactors (Actor|GetAllActorsOfClass "BasePlayerController_C"))
  (for _array_element _outactors
    (CallFunction|ToChat _array_element (Utilities|Text|ToText(String) (Utilities|String|Append (Utilities|String|ToString(Text) (Variables|Default|GetName)) ":" (Utilities|String|ToString(Text) Message))))))

(event Custom|To%20Chat
  (params (Message :type Text))
  (bind _ascustom_hud (Utilities|Casting|CastToCustomHUD (HUD|GetHUD)))
  (Utilities|IsValid (Default|GetWidgetbyClass _ascustom_hud "/Game/Blueprints/HUD/Chat.Chat_C")
    (:Is%20Valid
      (Default|NewMessage (.AsChat (Utilities|Casting|CastToChat (Default|GetWidgetbyClass _ascustom_hud "/Game/Blueprints/HUD/Chat.Chat_C"))) Message))))

(event Input|ActionEvents|InputActionChat
  (params (Key :type Key%20Structure :default "AnyKey"))
  (:Pressed
    (bind _ascustom_hud (Utilities|Casting|CastToCustomHUD (HUD|GetHUD)))
    (Utilities|IsValid (Default|GetWidgetbyClass _ascustom_hud "/Game/Blueprints/HUD/Chat.Chat_C")
      (:Is%20Valid
        (Input|SetInputModeUIOnly self (Default|GetWidgetbyClass _ascustom_hud "/Game/Blueprints/HUD/Chat.Chat_C") false)
        (Widget|SetKeyboardFocus (Default|GetWidgetbyClass _ascustom_hud "/Game/Blueprints/HUD/Chat.Chat_C"))))))

(fn ConstructionScript
  (Variables|Default|SetName (Utilities|Text|ToText(String) (Utilities|String|Append "Player-" (Utilities|String|ToString(Integer) (Math|Random|RandomIntegerinRange 1 9999))))))

(fn GetHudClasses
  (bind _classes (LocalVariables|GetClasses))
  (bind _asbase_character (Utilities|Casting|CastToBaseCharacter (Pawn|GetControlledPawn))
    (:then
      (Utilities|Array|AppendArray _classes (Default|GetWidgetClasses _asbase_character)))
    (:CastFailed
      _))
  (Utilities|Array|AppendArray _classes (Variables|Default|GetHUD%20Classes))
  (return _classes))