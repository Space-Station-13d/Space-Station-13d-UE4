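; Base first-person character that can walk, look, jump, interact with objects and carry one item at a time.
; Use finds the actor faced along the camera transform and calls OnInteract on each of its Interactable components.
; PickUp attaches an actor to the Hand socket with collision, physics and gravity off, while DropItem detaches it and restores them.
; It also exposes a list of HUD widget classes.
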(event `InputAxis|Forward`
  (params (AxisValue :type "Float (single-precision)"))
  ;[1 1 1] Movement
  (`self.AddMovementInput` (`self.GetActorForwardVector`) AxisValue))

(event `InputAxis|Look Down`
  (params (AxisValue :type "Float (single-precision)"))
  ;[1 1 1] Looking around
  (`self.AddControllerPitchInput` AxisValue))

(event `InputAxis|Look Right`
  (params (AxisValue :type "Float (single-precision)"))
  ;[1 1 1] Looking around
  (`self.AddControllerYawInput` AxisValue))

(event `InputAxis|Right`
  (params (AxisValue :type "Float (single-precision)"))
  ;[1 1 1] Movement
  (`self.AddMovementInput` (`self.GetActorRightVector`) AxisValue))

(event `InputAction|Jump`
  (params (Key :type "Key Structure" :default "AnyKey"))
  ;[1 1 1] Movement
  (:`Pressed`
    (`self.Jump`)))

(event `InputAction|Use`
  (params (Key :type "Key Structure" :default "AnyKey"))
  ;[1 1 1] Interaction
  (:`Pressed`
    (`self.Use` (`SceneComponent.K2_GetComponentToWorld` (`self.FirstPersonCamera`)))))

(event `Use`
  (params (Transform :type "Transform Structure"))
  (bind (_found _success) (`/Game/Blueprints/Libraries/Facing.Get Facing Actor` 2000.0 Transform))
  ;[1 1 1] Interaction
  (if _success
    (for _array_element (`self.K2_GetComponentsByClass` _found "/Script/SS13D_UE4_prototype.Interactable")
      (`Interactable.OnInteract` _array_element self))))

(event `InputAction|Drop`
  (params (Key :type "Key Structure" :default "AnyKey"))
  ;[1 1 1] Drop stuff
  (:`Pressed`
    (`self.Drop`)))

(event `Drop`
  ;[1 1 1] Drop stuff
  (`self.Drop Item`))

(fn `Drop Item`
  (bind _held_item (`self.Held Item`))
  (if (`self.Is Holding Item`)
    (`|ExecutionSequence`
      (:`then_0`
        (`self.DetachRootComponentFromParent` _held_item true))
      (:`then_1`
        (`self.SetActorEnableCollision` _held_item true))
      (:`then_2`
        (bind _asprimitive_component (cast `PrimitiveComponent` (`self.K2_GetRootComponent` _held_item)))
        (`|ExecutionSequence`
          (:`then_0`
            (`PrimitiveComponent.SetEnableGravity` _asprimitive_component true))
          (:`then_1`
            (`PrimitiveComponent.SetSimulatePhysics` _asprimitive_component true))))
      (:`then_3`
        (set `self.Is Holding Item` false)
        (set `self.Held Item` null)))))

(fn `Get Widget Classes`
  (returns (`Hud Classes` :type "Array of UserWidget Class Reference"))
  (return (`self.HUD Widget Classes`)))

(fn `Pick Up`
  (params (Actor :type "Actor Object Reference"))
  (bind _hand (`self.Hand`))
  (if (not (`self.Is Holding Item`))
    (`|ExecutionSequence`
      (:`then_0`
        (`self.K2_AttachRootComponentTo` Actor _hand "Hand" "KeepWorldPosition" true)
        (`KismetSystemLibrary.PrintString` "hi"))
      (:`then_1`
        (`self.K2_SetActorLocation` Actor (`SceneComponent.GetSocketLocation` _hand "Hand") false false)
        (`self.SetActorEnableCollision` Actor false)
        (bind _asprimitive_component (cast `PrimitiveComponent` (`self.K2_GetRootComponent` Actor)))
        (`PrimitiveComponent.SetSimulatePhysics` _asprimitive_component false)
        (`PrimitiveComponent.SetEnableGravity` _asprimitive_component false))
      (:`then_2`
        (set `self.Is Holding Item` true)
        (set `self.Held Item` Actor)))))

(fn `UserConstructionScript`)